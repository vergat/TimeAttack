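; Player vehicle for a time attack race that stays without input until the race starts and respawns when it gets stuck.
; BeginPlay stores its transform as the respawn location on the player controller, whose RaceStart flag gates input and the parent Tick.
; During the race, Tick destroys the vehicle if it is upside-down or on its side at low speed, confirmed again after a short delay.
; On destruction, it asks the controller to respawn it.
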(event EventDestroyed
  ;[1 1 1] Respawn vehicle
  (Default|RespawnVehicle (Variables|Default|GetPlayerController)))

(event EventBeginPlay
  (|CallParentFunction)
  ;[1 1 1] Initialize respawn location
  (bind _astime_attack_player_controller_old_bp (Utilities|Casting|CastToTimeAttackPlayerControllerOldBP (Game|GetPlayerController 0)))
  (bind _output_get (Variables|Default|SetPlayerController _astime_attack_player_controller_old_bp))
  (Variables|/Game/TimeAttack/Blueprints/TimeAttackPlayerControllerOldBP.TimeAttackPlayerControllerOldBP_C|SetRespawnLocation _output_get (Transformation|GetActorTransform))
  ;[1 1 1] Disable input - It wil be enabled when the race starts
  (Input|DisableInput (Variables|Default|GetPlayerController)))

(event EventTick
  (params (DeltaSeconds :type Float%20%28single-precision%29))
  (bind _playercontroller (Variables|Default|GetPlayerController))
  ;[1 1 1] Enable input only after race start
  (if (Variables|/Game/TimeAttack/Blueprints/TimeAttackPlayerControllerOldBP.TimeAttackPlayerControllerOldBP_C|GetRaceStart _playercontroller)
    (Input|EnableInput _playercontroller)
    (|CallParentFunction DeltaSeconds)
    ;[1 1 1] Check if upside-down and self-destroy in order to respawn
    (bind _mustberespawned (CallFunction|RespawnCheck))
    (if _mustberespawned
      (Utilities|FlowControl|Delay 2.0)
      (bind _mustberespawned_2 (CallFunction|RespawnCheck))
      (if _mustberespawned_2
        (Actor|DestroyActor)))))

(fn ConstructionScript)

(fn RespawnCheck
  ;[1 1 1] Check if you are upside-down and low-speed
  (bind _output_get (Variables|Default|SetIsStuck (and (< (Math|Vector|DotProduct (Transformation|GetActorUpVector) "0, 0,1.000000") 0.5) (< (Class|WheeledVehicleMovementComponent|GetForwardSpeed (Variables|Default|GetVehicleMovement)) 0.5))))
  (return _output_get))