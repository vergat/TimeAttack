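; Player controller for a time-attack racing mode that runs the splash screen, countdown, lap and race timing, vehicle respawn and level restart.
; A click starts the countdown, then timelines drive the lap and race clocks as text for the TimeAttackHUDBP widget.
; Lap updates compare times against the bests and write records to a save slot.
; R or right-click resets saved bests before the race starts.
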(event Custom|Setup
  ;[1 1 1] Load an existring savegame, if any or create a new one
  (CallFunction|SaveGameCheck)
  ;[1 1 1] Refresh HUD text
  (CallFunction|RefreshHUD))

(event Custom|Restart
  ;[1 1 1] Restart map when the race is completed
  (Variables|Status|SetRaceStart false)
  (Utilities|FlowControl|Delay 5.0)
  (Development|ExecuteConsoleCommand "RestartLevel"))

(event Custom|UpdateLap
  ;[1 1 1] Do you have completed the race?
  (if (Variables|Status|GetRaceComplete)
    _
    (else
      ;[1 1 1] Update lap counter
      (bind _output_get (Variables|Values|SetCurrentLap (+ (Variables|Values|GetCurrentLap) 1)))
      (Variables|Text|SetCurrentLapText (Utilities|Text|ToText(Integer) _output_get))))
  ;[1 1 1] Update lap/race time
  (CallFunction|EndLapUpdate))

(event Custom|StartRaceTime
  ;[1 1 1] Manage Race Time
  (bind _time (Timeline|GameTime Play)
    (:Update
      (bind _output_get (Variables|Values|SetCurrentRaceTime _time))
      (Variables|Text|SetCurrentRaceTimeText (Utilities|TimetoText _output_get)))))

(event Custom|StopRaceTime
  ;[1 1 1] Manage Race Time
  (bind _time (Timeline|GameTime Stop)
    (:Update
      (bind _output_get (Variables|Values|SetCurrentRaceTime _time))
      (Variables|Text|SetCurrentRaceTimeText (Utilities|TimetoText _output_get)))))

(event Custom|StartLapTime
  ;[1 1 1] Maage Lap Time
  (bind _time (Timeline|Timeline_0 PlayFromStart)
    (:Update
      (bind _output_get (Variables|Values|SetCurrentLapTime _time))
      (Variables|Text|SetCurrentLapTimeText (Utilities|TimetoText _output_get)))))

(event Custom|StopLapTime
  ;[1 1 1] Maage Lap Time
  (bind _time (Timeline|Timeline_0 Stop)
    (:Update
      (bind _output_get (Variables|Values|SetCurrentLapTime _time))
      (Variables|Text|SetCurrentLapTimeText (Utilities|TimetoText _output_get)))))

(event Custom|RespawnVehicle
  ;[1 1 1] Vehicle respawn
  (bind _returnvalue (Game|SpawnActorfromClass "/Game/TimeAttack/Blueprints/TimeAttackVehicle.TimeAttackVehicle_C" (Variables|Respawn|GetRespawnLocation) "Undefined" 0 0))
  (Pawn|Possess _returnvalue))

(event EventBeginPlay
  ;[1 1 1] Get a reference to current pawn
  (bind _astime_attack_pawn (Utilities|Casting|CastToTimeAttackPawn (Game|Player|GetPlayerPawn 0)))
  (Variables|References|SetVehicle _astime_attack_pawn)
  ;[1 1 1] Spawn game-mode specific HUD
  (bind _returnvalue (UserInterface|CreateWidget "/Game/TimeAttack/Blueprints/TimeAttackHUDBP.TimeAttackHUDBP_C"))
  (bind _output_get (Variables|References|SetHUD _returnvalue))
  (UserInterface|Viewport|AddtoViewport _output_get 0)
  ;[1 1 1] Set initial panels visibiliy
  (Variables|/Game/TimeAttack/Blueprints/TimeAttackHUDBP.TimeAttackHUDBP_C|SetSplashScreenVisible _output_get "Visible")
  (Variables|/Game/TimeAttack/Blueprints/TimeAttackHUDBP.TimeAttackHUDBP_C|SetCountdownVisible _output_get "Hidden")
  (Variables|/Game/TimeAttack/Blueprints/TimeAttackHUDBP.TimeAttackHUDBP_C|SetGameHUDVisible _output_get "Hidden")
  ;[1 1 1] Initialize status
  (Variables|Values|SetCurrentLap 1))

(event Input|KeyboardEvents|R
  (params (Key :type Key%20Structure :default "AnyKey"))
  ;[1 1 1] Reset best time when you press 'R' during the splash screen
  (:Pressed
    (if (not (Variables|Status|GetRaceStart))
      (Variables|Values|SetBestLapTime (Variables|Values|GetDefaultBestLapTime))
      (Variables|Values|SetBestRaceTime (Variables|Values|GetDefaultBestRaceTime))
      (CallFunction|SaveGame)
      (CallFunction|RefreshHUD))))

(event Input|KeyboardEvents|P
  (params (Key :type Key%20Structure :default "AnyKey"))
  ;[1 0 0] Debug only - Log timers
  (:Pressed
    (Variables|Text|SetBestLapTimeText (Utilities|TimetoText (Variables|Values|GetBestLapTime)))
    (Variables|Text|SetBestRaceTimeText (Utilities|TimetoText (Variables|Values|GetBestRaceTime)))
    (Development|PrintText (Variables|Text|GetBestLapTimeText))
    (Development|PrintText (Variables|Text|GetBestRaceTimeText))))

(event Input|MouseEvents|LeftMouseButton
  (params (Key :type Key%20Structure :default "AnyKey"))
  (bind _hud (Variables|References|GetHUD))
  (bind _hud_2 (Variables|References|GetHUD))
  ;[0 1 0] Start race sequence
  (:Pressed
    (Utilities|FlowControl|DoOnce false
      (:Completed
        ;;[1 1 1] Hide SplashScreen
        (Variables|/Game/TimeAttack/Blueprints/TimeAttackHUDBP.TimeAttackHUDBP_C|SetSplashScreenVisible _hud "Hidden")
        ;;[1 1 1] Show Countdown
        (Variables|/Game/TimeAttack/Blueprints/TimeAttackHUDBP.TimeAttackHUDBP_C|SetCountdownVisible _hud "Visible")
        ;;[1 1 1] Countdown sequence
        (Variables|Text|SetCountdownText "3")
        (Utilities|FlowControl|Delay 2.5)
        (Variables|Text|SetCountdownText "2")
        (Utilities|FlowControl|Delay 1.0)
        (Variables|Text|SetCountdownText "1")
        (Utilities|FlowControl|Delay 1.0)
        (Variables|Text|SetCountdownText "GO!")
        (Utilities|FlowControl|Delay 1.0)
        ;;[1 1 1] Hide Countdown
        (Variables|/Game/TimeAttack/Blueprints/TimeAttackHUDBP.TimeAttackHUDBP_C|SetCountdownVisible _hud_2 "Hidden")
        ;;[1 1 1] Show GameHUD
        (Variables|/Game/TimeAttack/Blueprints/TimeAttackHUDBP.TimeAttackHUDBP_C|SetGameHUDVisible _hud_2 "Visible")
        ;;[1 1 1] Start Race
        (Variables|Status|SetRaceStart true)
        (CallFunction|StartRaceTime)
        (CallFunction|StartLapTime)))))

(event Input|MouseEvents|RightMouseButton
  (params (Key :type Key%20Structure :default "AnyKey"))
  ;[1 1 1] Reset best time when you press 'R' during the splash screen
  (:Pressed
    (if (not (Variables|Status|GetRaceStart))
      (Variables|Values|SetBestLapTime (Variables|Values|GetDefaultBestLapTime))
      (Variables|Values|SetBestRaceTime (Variables|Values|GetDefaultBestRaceTime))
      (CallFunction|SaveGame)
      (CallFunction|RefreshHUD))))

(fn ConstructionScript)

(fn RefreshHUD
  ;[1 1 1] Convert numerical values into text for the HUD
  (Variables|Text|SetCurrentLapText (Utilities|Text|ToText(Integer) (Variables|Values|GetCurrentLap)))
  (Variables|Text|SetMaxLapsText (Utilities|Text|ToText(Integer) (Variables|Values|GetMaxLaps)))
  (Variables|Text|SetGoldTimeText (Utilities|TimetoText (Variables|Values|GetGoldTime)))
  (Variables|Text|SetSilverTimeText (Utilities|TimetoText (Variables|Values|GetSilverTime)))
  (Variables|Text|SetBronzeTimeText (Utilities|TimetoText (Variables|Values|GetBronzeTime)))
  (Variables|Text|SetBestLapTimeText (Utilities|TimetoText (Variables|Values|GetBestLapTime)))
  (Variables|Text|SetBestRaceTimeText (Utilities|TimetoText (Variables|Values|GetBestRaceTime))))

(fn SaveGameCheck
  ;[1 1 1] Check if a savegame exists
  (bind _returnvalue (SaveGame|DoesSaveGameExist (Variables|Saves|GetSaveSlot)))
  (if _returnvalue
    ;[1 1 1] Load it!
    (CallFunction|LoadGame)
    (else
      ;[1 1 1] Create a new savegame with default best times
      (Variables|Values|SetBestLapTime (Variables|Values|GetDefaultBestLapTime))
      (Variables|Values|SetBestRaceTime (Variables|Values|GetDefaultBestRaceTime))
      (CallFunction|SaveGame))))

(fn SaveGame
  ;[1 1 1] Create a new savegame and save it into the specified SaveSlot
  (bind _returnvalue (SaveGame|CreateSaveGameObject "/Game/TimeAttack/Blueprints/TimeAttackSaveGame.TimeAttackSaveGame_C"))
  (bind _output_get (Variables|Saves|SetSaveGameReference _returnvalue))
  (Variables|/Game/TimeAttack/Blueprints/TimeAttackSaveGame.TimeAttackSaveGame_C|SetSavedBestLapTime _output_get (Variables|Values|GetBestLapTime))
  (Variables|/Game/TimeAttack/Blueprints/TimeAttackSaveGame.TimeAttackSaveGame_C|SetSavedBestRaceTime _output_get (Variables|Values|GetBestRaceTime))
  (SaveGame|SaveGametoSlot (Variables|Saves|GetSaveGameReference) (Variables|Saves|GetSaveSlot)))

(fn LoadGame
  ;[1 1 1] Load best times from the specified SaveSlot
  (bind _returnvalue (SaveGame|LoadGamefromSlot (Variables|Saves|GetSaveSlot)))
  (bind _astime_attack_save_game (Utilities|Casting|CastToTimeAttackSaveGame _returnvalue))
  (Variables|Values|SetBestLapTime (Variables|/Game/TimeAttack/Blueprints/TimeAttackSaveGame.TimeAttackSaveGame_C|GetSavedBestLapTime _astime_attack_save_game))
  (Variables|Values|SetBestRaceTime (Variables|/Game/TimeAttack/Blueprints/TimeAttackSaveGame.TimeAttackSaveGame_C|GetSavedBestRaceTime _astime_attack_save_game)))

(fn EndLapUpdate
  ;[0 0 1 0.5] Update lap/race time - This function is called during each end-lap
  ;;[1 1 1] Reset lap timer
  (CallFunction|StopLapTime)
  ;;[1 1 1] Is it a new best Lap Time?
  (if (<= (Variables|Values|GetCurrentLapTime) (Variables|Values|GetBestLapTime))
    ;;[1 1 1] Update actual best Lap Time
    (bind _output_get (Variables|Values|SetBestLapTime (Variables|Values|GetCurrentLapTime)))
    (Variables|Text|SetBestLapTimeText (Utilities|TimetoText _output_get))
    ;;[1 1 1] Save new results
    (CallFunction|SaveGame))
  ;;[1 1 1] Reset current lap time
  (Variables|Values|SetCurrentLapTime 0.0)
  ;;[1 1 1] Is race completed?
  (if (Variables|Status|GetRaceComplete)
    ;;[1 1 1] Update Race Time and check for a new record
    (CallFunction|EndRaceUpdate)
    (else
      ;;[1 1 1] Re-start lap timer
      (CallFunction|StartLapTime))))

(fn EndRaceUpdate
  ;[1 1 1] Is a new best Race Time?
  (if (< (Variables|Values|GetCurrentRaceTime) (Variables|Values|GetBestRaceTime))
    ;[1 1 1] Update actual best Race Time
    (bind _output_get (Variables|Values|SetBestRaceTime (Variables|Values|GetCurrentRaceTime)))
    (Variables|Text|SetBestRaceTimeText (Utilities|TimetoText _output_get))
    ;[1 1 1] Save new results
    (CallFunction|SaveGame)))