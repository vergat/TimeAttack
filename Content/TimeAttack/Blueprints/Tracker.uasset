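; Time attack track manager that runs a lap-based checkpoint race for the player.
; On BeginPlay it pushes medal times, lap count, map name and save slot into the player controller, then indexes the checkpoint array, activates only the first and binds their passed events.
; Each pass updates the respawn transform and activates the next checkpoint; the last one updates the lap, looping to the first or restarting once the race completes.
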(event Custom|SetupCheckpoints
  (bind _checkpoints (Variables|Checkpoints|GetCheckpoints))
  ;[1 1 1] Assign checkpoint indices
  (for (_array_element _array_index) (Variables|Checkpoints|GetCheckpoints)
    (Variables|/Game/TimeAttack/Blueprints/Checkpoint.Checkpoint_C|SetCheckpointIndex _array_element _array_index))
  ;[1 1 1] Compute total checkpoints count
  (Variables|Checkpoints|SetTotalCheckpoints (Utilities|Array|Length _checkpoints))
  ;[1 1 1] Start with all checkpoints deactivated
  (for _array_element_2 _checkpoints
    (Utils|DeactivateCheckpoint _array_element_2))
  ;[1 1 1] Activate the first checkpoint
  (Utils|ActivateCheckpoint (Utilities|Array|Get(acopy) _checkpoints))
  ;[1 1 1] Bind "OnCheckpointPassed" event to all registered checkpoints
  (for _array_element_3 _checkpoints
    (EventDispatchers|BindEventtoCheckpointPassed _array_element_3 (delegate Custom|OnCheckpointPassed))))

(event Custom|OnCheckpointPassed
  (params (CheckpointIndex :type Integer))
  (bind _playercontroller (Variables|References|GetPlayerController))
  ;[1 1 1] Update lap counter/timers and manage checkpoints
  (RaceLogic|LapCheck CheckpointIndex)
  ;[1 1 1] If you have completed the race, restart game
  (if (Variables|/Game/TimeAttack/Blueprints/TimeAttackPlayerControllerOldBP.TimeAttackPlayerControllerOldBP_C|GetRaceComplete _playercontroller)
    (Default|Restart _playercontroller)))

(event EventBeginPlay
  ;[1 1 1] Get a reference to current PlayerController
  (bind _astime_attack_player_controller_old_bp (Utilities|Casting|CastToTimeAttackPlayerControllerOldBP (Game|GetPlayerController 0)))
  (bind _output_get (Variables|References|SetPlayerController _astime_attack_player_controller_old_bp))
  ;[1 1 1] Setup PlayerController
  (Setup|SetupPlayerController _output_get)
  ;[1 1 1] Setup race checkpoints
  (CallFunction|SetupCheckpoints))

(fn ConstructionScript)

(fn SetupPlayerController
  (params (TargetPlayer :type Time%20Attack%20Player%20Controller%20Old%20BP%20Object%20Reference))
  (bind _playercontroller (Variables|References|GetPlayerController))
  ;[1 1 1] Set reference times
  (Variables|/Game/TimeAttack/Blueprints/TimeAttackPlayerControllerOldBP.TimeAttackPlayerControllerOldBP_C|SetGoldTime _playercontroller (Variables|RaceSettings|GetGoldTime))
  (Variables|/Game/TimeAttack/Blueprints/TimeAttackPlayerControllerOldBP.TimeAttackPlayerControllerOldBP_C|SetSilverTime _playercontroller (Variables|RaceSettings|GetSilverTime))
  (Variables|/Game/TimeAttack/Blueprints/TimeAttackPlayerControllerOldBP.TimeAttackPlayerControllerOldBP_C|SetBronzeTime _playercontroller (Variables|RaceSettings|GetBronzeTime))
  (Variables|/Game/TimeAttack/Blueprints/TimeAttackPlayerControllerOldBP.TimeAttackPlayerControllerOldBP_C|SetDefaultBestLapTime _playercontroller (Variables|RaceSettings|GetDefaultBestLap))
  (Variables|/Game/TimeAttack/Blueprints/TimeAttackPlayerControllerOldBP.TimeAttackPlayerControllerOldBP_C|SetDefaultBestRaceTime _playercontroller (Variables|RaceSettings|GetDefaultBestTime))
  ;[1 1 1] Set reference laps
  (Variables|/Game/TimeAttack/Blueprints/TimeAttackPlayerControllerOldBP.TimeAttackPlayerControllerOldBP_C|SetMaxLaps _playercontroller (Variables|RaceSettings|GetMaxLaps))
  ;[1 1 1] Set map name
  (Variables|/Game/TimeAttack/Blueprints/TimeAttackPlayerControllerOldBP.TimeAttackPlayerControllerOldBP_C|SetMapName _playercontroller (Variables|CustomSettings|GetMapName))
  ;[1 1 1] Set save slot
  (Variables|/Game/TimeAttack/Blueprints/TimeAttackPlayerControllerOldBP.TimeAttackPlayerControllerOldBP_C|SetSaveSlot _playercontroller (Variables|CustomSettings|GetSaveGameName))
  ;[1 1 1] Setup PlayerController
  (Default|Setup _playercontroller))

(fn LapCheck
  (params (CheckpointPassed :type Integer))
  ;[1 1 1] Cache this checkpoint index
  (LocalVariables|SetCheckpointIndex CheckpointPassed)
  ;[1 1 1] Update your current respawn location
  (Variables|/Game/TimeAttack/Blueprints/TimeAttackPlayerControllerOldBP.TimeAttackPlayerControllerOldBP_C|SetRespawnLocation (Variables|References|GetPlayerController) (Transformation|GetActorTransform (Utilities|Array|Get(acopy) (Variables|Checkpoints|GetCheckpoints) (LocalVariables|GetCheckpointIndex))))
  ;[1 1 1] Check if you have passed the last checkpoint
  (if (== (LocalVariables|GetCheckpointIndex) (- (Variables|Checkpoints|GetTotalCheckpoints) 1))
    ;[1 1 1] Do you have completed the race?
    (bind _isracecomplete (RaceLogic|RaceCompleteCheck))
    (if _isracecomplete
      _
      (else
        ;[1 1 1] Activate the next checkpoint (0)
        (Utils|ActivateCheckpoint (Utilities|Array|Get(acopy) (Variables|Checkpoints|GetCheckpoints)))))
    ;[1 1 1] Update lap counter and timer
    (Default|UpdateLap (Variables|References|GetPlayerController))
    (else
      ;[1 1 1] Activate the next checkpoint
      (Utils|ActivateCheckpoint (Utilities|Array|Get(acopy) (Variables|Checkpoints|GetCheckpoints) (+ (LocalVariables|GetCheckpointIndex) 1))))))

(fn ActivateCheckpoint
  (params (TargetCheckpoint :type Checkpoint%20Object%20Reference))
  (Default|Activate TargetCheckpoint))

(fn DeactivateCheckpoint
  (params (TargetCheckpoint :type Checkpoint%20Object%20Reference))
  (Default|Deactivate TargetCheckpoint))

(fn RaceCompleteCheck
  (bind _playercontroller (Variables|References|GetPlayerController))
  ;[1 1 1] Do you have completed the last lap?
  (bind _output_get (Variables|/Game/TimeAttack/Blueprints/TimeAttackPlayerControllerOldBP.TimeAttackPlayerControllerOldBP_C|SetRaceComplete (Variables|References|GetPlayerController) (>= (Variables|/Game/TimeAttack/Blueprints/TimeAttackPlayerControllerOldBP.TimeAttackPlayerControllerOldBP_C|GetCurrentLap _playercontroller) (Variables|/Game/TimeAttack/Blueprints/TimeAttackPlayerControllerOldBP.TimeAttackPlayerControllerOldBP_C|GetMaxLaps _playercontroller))))
  (return _output_get))